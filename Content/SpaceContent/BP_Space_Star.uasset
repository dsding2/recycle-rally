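; BP_Space_Star is a star actor that exerts gravity on nearby physics objects and destroys first-person projectiles that hit it.
; Every tick it queries PhysicsBody actors overlapping its GravityCollision component.
; Those with a static mesh root receive a force toward the star's location, using a fixed strength with inverse-square distance falloff.
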(event EventBeginPlay)

(event Collision|EventActorBeginOverlap
  (params (OtherActor :type Actor%20Object%20Reference)))

(event Collision|EventHit
  (params (MyComp :type Primitive%20Component%20Object%20Reference) (Other :type Actor%20Object%20Reference) (OtherComp :type Primitive%20Component%20Object%20Reference) (bSelfMoved :type Boolean) (HitLocation :type Vector :default "0, 0, 0") (HitNormal :type Vector :default "0, 0, 0") (NormalImpulse :type Vector :default "0, 0, 0") (Hit :type Hit%20Result%20Structure%20%28by%20ref%29))
  (bind _asbp_first_person_projectile (Utilities|Casting|CastToBP_FirstPersonProjectile Other))
  (Actor|DestroyActor _asbp_first_person_projectile))

(event EventTick
  (params (DeltaSeconds :type Float%20%28single-precision%29))
  (bind _outactors (Collision|ComponentOverlapActors (Variables|Default|GetGravity%20Collision) (Transformation|GetActorTransform) (Utilities|Array|MakeArray (Utilities|Enum|LiteralenumEObjectTypeQuery "ObjectTypeQuery4")) "/Script/Engine.Actor"))
  (for _array_element _outactors
    (bind _asstatic_mesh_component (Utilities|Casting|CastToStaticMeshComponent (Variables|/Script/Engine.Actor|GetRootComponent _array_element)))
    (Physics|AddForce _asstatic_mesh_component (* (/ (Math|Vector|Normalize (- (Transformation|GetActorLocation) (Transformation|GetActorLocation _array_element))) (Math|Vector|VectorLengthSquared (- (Transformation|GetActorLocation) (Transformation|GetActorLocation _array_element)))) 5e+09) "None" false)))

(fn ConstructionScript)