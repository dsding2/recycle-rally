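; BP_Spacebasket is a space prop that tumbles and shrinks as it is pulled toward the black hole.
; On BeginPlay it caches the vector to BP_Space_Black_Hole and gives its static mesh a huge random torque for spin.
; Each Tick applies acceleration along that fixed, unnormalized vector, so initial distance sets the pull strength.
; Scale drops by a constant step per frame, independent of delta time and without a lower limit.
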(event EventBeginPlay
  (bind _returnvalue (Actor|GetActorOfClass "/Game/SpaceContent/BP_Space_Black_Hole.BP_Space_Black_Hole_C"))
  (Variables|Default|SetGravityVector (- (Transformation|GetActorLocation _returnvalue) (Transformation|GetActorLocation)))
  (Class|PrimitiveComponent|AddTorqueinDegrees (Variables|Default|GetStaticMesh) (* (Math|Random|RandomUnitVector) 1e+09) "None" false))

(event Collision|EventActorBeginOverlap
  (params (OtherActor :type Actor%20Object%20Reference)))

(event EventTick
  (params (DeltaSeconds :type Float%20%28single-precision%29))
  (Transformation|SetActorScale3D (- (Transformation|GetActorScale3D) "0.010000,0.010000,0.010000"))
  (Physics|AddForce (Variables|Default|GetStaticMesh) (* (Variables|Default|GetGravityVector) 0.5) "None" true))

(fn ConstructionScript)