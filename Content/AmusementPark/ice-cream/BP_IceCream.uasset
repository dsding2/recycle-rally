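; BP_IceCream is an ice cream actor in the amusement park that reacts when the first-person player touches it.
; An overlap on the Ice_Cream_01_ component, filtered by a cast to BP_FirstPersonCharacter, randomly picks one of two splash UI widgets.
; The chosen widget shows briefly on the viewport, then is removed and the ice cream destroys itself.
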(event OnComponentBeginOverlap(Ice_Cream_01_)
  (params (OverlappedComponent :type Primitive%20Component%20Object%20Reference) (OtherActor :type Actor%20Object%20Reference) (OtherComp :type Primitive%20Component%20Object%20Reference) (OtherBodyIndex :type Integer) (bFromSweep :type Boolean) (SweepResult :type Hit%20Result%20Structure%20%28by%20ref%29))
  (Utilities|Casting|CastToBP_FirstPersonCharacter OtherActor)
  (switch int (Math|Conversions|ToInteger(Byte) (Class|KismetMathLibrary|RandomInteger64inRange 0 1))
    (:0
      (bind _returnvalue (UserInterface|CreateWidget "/Game/AmusementPark/ice-cream/UI_splash.UI_splash_C"))
      (UserInterface|Viewport|AddtoViewport _returnvalue 0)
      (Utilities|FlowControl|Delay 1.0)
      (Widget|RemovefromParent _returnvalue)
      (Actor|DestroyActor))
    (:1
      (bind _returnvalue_2 (UserInterface|CreateWidget "/Game/AmusementPark/ice-cream/UI_splash2.UI_splash2_C"))
      (UserInterface|Viewport|AddtoViewport _returnvalue_2 0)
      (Utilities|FlowControl|Delay 1.0)
      (Widget|RemovefromParent _returnvalue_2)
      (Actor|DestroyActor))))

(event EventBeginPlay)

(event Collision|EventActorBeginOverlap
  (params (OtherActor :type Actor%20Object%20Reference)))

(event EventTick
  (params (DeltaSeconds :type Float%20%28single-precision%29)))

(fn ConstructionScript)