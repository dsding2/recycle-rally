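; BP_IceCreamThrower is an amusement park actor that throws ice cream by repeatedly spawning BP_IceCream actors.
; BeginPlay starts the Throw custom event after a short delay.
; Throw prints a debug string, spawns the ice cream at the ProjectileSpawn component's world transform, then waits a random whole number of seconds before calling itself, forming an endless loop without Tick.
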(event Custom|Throw
  (Development|PrintString "Throw")
  (Game|SpawnActorfromClass "/Game/AmusementPark/ice-cream/BP_IceCream.BP_IceCream_C" (Transformation|GetWorldTransform (Variables|Default|GetProjectile%20Spawn)) "Undefined" "MultiplyWithRoot" 0 0)
  (Utilities|FlowControl|Delay (Math|Conversions|ToFloat(Integer) (Class|KismetMathLibrary|RandomInteger64inRange 2 10)))
  (CallFunction|Throw))

(event EventBeginPlay
  (Utilities|FlowControl|Delay 2.0)
  (CallFunction|Throw))

(event Collision|EventActorBeginOverlap
  (params (OtherActor :type Actor%20Object%20Reference)))

(event EventTick
  (params (DeltaSeconds :type Float%20%28single-precision%29)))

(fn ConstructionScript)